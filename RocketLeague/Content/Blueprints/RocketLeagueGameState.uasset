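; Game state for a Rocket League-style match, tracking the countdown clock and Blue and Red team goals.
; InitializeMatch derives the clock from the game mode's match length, resets scores, has the local player controller spawn and add its HUD, and spawns the ball on authority.
; Tick drives a delay-based one-second countdown; at zero the game pauses, prints the winner or draw, then requests a delayed quit.
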(event `InitializeMatch`
  ;[1 1 1] Set minutes and seconds for match, Spawn Actors
  (`|ExecutionSequence`
    (:`then_0`
      (bind _asrocket_league_game_mode_bp (cast `/Game/Blueprints/RocketLeagueGameMode_BP` (`GameplayStatics.GetGameMode`)))
      (bind (_remainder _returnvalue) (`KismetMathLibrary.FMod` (`KismetMathLibrary.Conv_IntToDouble` (`/Game/Blueprints/RocketLeagueGameMode_BP.MatchLength` _asrocket_league_game_mode_bp)) 60.0))
      (set `self.Minutes` _returnvalue)
      (set `self.Seconds` (`KismetMathLibrary.FTrunc` _remainder))
      (set `self.BlueTeamGoals` 0)
      (set `self.RedTeamGoals` 0))
    (:`then_1`
      (bind _asrocket_league_player_controller (cast `/Game/Blueprints/Gameplay/Vehicle/RocketLeaguePlayerController` (`GameplayStatics.GetPlayerController` 0)))
      (set `self.PlayerControllerRef` _asrocket_league_player_controller))
    (:`then_2`
      (`self.SpawnActors`)
      (`self.SpawnBall`)
      (`self.SetActorTickEnabled` true))))

(event `SpawnBall`
  ;[1 1 1] Spawn the ball
  (if (== (`self.BallRef`) null)
    (`/Engine/EditorBlueprintResources/ActorMacros.Switch Has Authority`
      (:`Authority`
        (bind _returnvalue (`|SpawnActorFromClass` "/Game/Blueprints/Gameplay/Ball/Ball.Ball_C" (`self.BallSpawnTransform`) "Undefined" "OverrideRootScale" null null))
        (`KismetSystemLibrary.Delay` 0.2)
        (`/Engine/EditorBlueprintResources/StandardMacros.IsValid` _returnvalue
          (:`Is Valid`
            (set `self.BallRef` _returnvalue)))))))

(event `SpawnActors`
  (bind _playercontrollerref (`self.PlayerControllerRef`))
  ;[1 1 1] Spawn Actors
  (`/Game/Blueprints/Gameplay/Vehicle/RocketLeaguePlayerController.Spawn` _playercontrollerref)
  (`/Game/Blueprints/Gameplay/Vehicle/RocketLeaguePlayerController.AddHUD` _playercontrollerref))

(event `Kickoff`)

(event `self.ReceiveTick`
  (params (DeltaSeconds :type "Float (single-precision)"))
  ;[1 1 1] Constantly check Match State
  (bind _time_is_up_ (`self.DecrementTimer`)
    (:`Out`
      (if _time_is_up_
        (`self.SetActorTickEnabled` (not _time_is_up_))
        (`self.EndGame`)))))

(event `BlueScored`
  ;[1 1 1] Scoring
  (`/Engine/EditorBlueprintResources/StandardMacros.IncrementInt` (`self.BlueTeamGoals`)
    (:`  `
      (`KismetSystemLibrary.PrintString` "Blue Team Scord!" true false (struct :`G` 0.66 :`B` 1.0 :`A` 1.0) 5.0))))

(event `RedScored`
  ;[1 1 1] Scoring
  (`/Engine/EditorBlueprintResources/StandardMacros.IncrementInt` (`self.RedTeamGoals`)
    (:`  `
      (`KismetSystemLibrary.PrintString` "Read Team Scord!" true false (struct :`R` 1.0 :`G` 0.068703 :`B` 0.106404 :`A` 1.0) 5.0))))

(event `EndGame`
  ;[1 1 1] Handle the game ending, display winner and quit
  (`GameplayStatics.SetGamePaused` true)
  (`self.DisplayWinner`
    (:`Out`
      (`KismetSystemLibrary.Delay` 5.0)
      (`KismetSystemLibrary.QuitGame` (`self.PlayerControllerRef`) "Quit"))))

(fn `UserConstructionScript`)